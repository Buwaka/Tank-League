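; TankUnit holds both players' hovering tanks in one Blueprint, handling movement and shooting for local two-player control.
; Each Tick teleports both bodies to HoverHeight, then applies forward and yaw impulses from input, with turning scaled by forward input.
; Shoot presses set flags that Tick consumes, spawning one Bullet at the tank's socket and launching it forward by impulse.
; SetStartTransforms stores and applies both starting transforms.
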(event EventTick
  (params (DeltaSeconds :type Float%20%28single-precision%29))
  (bind _returnvalue (Input|AxisValues|Getp1forward))
  (bind _returnvalue_2 (Input|AxisValues|Getp2forward))
  (bind _player_2 (Variables|Default|GetPlayer%202))
  (bind _player_1 (Variables|Default|GetPlayer%201))
  (bind _player_1_2 (Variables|Default|GetPlayer%201))
  (bind _player_1_3 (Variables|Default|GetPlayer%201))
  (bind _player_2_2 (Variables|Default|GetPlayer%202))
  (bind _player_2_3 (Variables|Default|GetPlayer%202))
  (bind _returnvalue_3 (Transformation|GetWorldLocation _player_2))
  (bind _returnvalue_4 (Transformation|GetWorldLocation _player_1_2))
  (bind _returnvalue_5 (Transformation|GetWorldTransform _player_2_2))
  (bind _returnvalue_6 (Transformation|GetWorldTransform _player_1_3))
  (bind (_x _y _z) (Math|Vector|BreakVector _returnvalue_3))
  (bind (_x_2 _y_2 _z_2) (Math|Vector|BreakVector _returnvalue_4))
  (bind (_location _rotation _scale) (Math|Transform|BreakTransform _returnvalue_5))
  (bind (_location_2 _rotation_2 _scale_2) (Math|Transform|BreakTransform _returnvalue_6))
  (Utilities|FlowControl|Sequence
    (:then_0
      (Utilities|FlowControl|Sequence
        (:then_0
          ;[1 1 1] hovering
          (Transformation|SetWorldLocation _player_1_2 (Math|Vector|MakeVector _x_2 _y_2 (Variables|Default|GetHover%20height)) false true))
        (:then_1
          ;[1 1 1] forward acceleration
          (Physics|AddImpulse _player_1 (* (Math|Vector|GetForwardVector _player_1) (* (Variables|Default|Getspeed) _returnvalue)) "None" true))
        (:then_2
          ;[1 1 1] rotation
          (Class|PrimitiveComponent|AddAngularImpulseinDegrees _player_1 (Math|Vector|MakeVector 0.0 0.0 (* _returnvalue (Input|AxisValues|Getp1right) (Variables|Default|Getturningspeed))) "None" true))
        (:then_3
          ;[1 1 1] Shoot
          (if (Variables|Default|Getp1%20shoot)
            (bind _returnvalue_7 (Game|SpawnActorfromClass "/Game/Blueprints/bullet.bullet_C" (Math|Transform|MakeTransform (Transformation|GetSocketLocation _player_1_3 "Bullet") _rotation_2 _scale_2) "Undefined" 0 0))
            (Physics|AddImpulse (Variables|/Game/Blueprints/bullet.bullet_C|GetSphere _returnvalue_7) (* (Math|Vector|GetForwardVector _player_1_3) (Variables|Default|GetshootForce)) "None" true)
            (Variables|Default|Setp1%20shoot false)))))
    (:then_1
      (Utilities|FlowControl|Sequence
        (:then_0
          (Transformation|SetWorldLocation _player_2 (Math|Vector|MakeVector _x _y (Variables|Default|GetHover%20height)) false true))
        (:then_1
          (Physics|AddImpulse _player_2_3 (* (Math|Vector|GetForwardVector _player_2_3) (* (Variables|Default|Getspeed) _returnvalue_2)) "None" true))
        (:then_2
          (Class|PrimitiveComponent|AddAngularImpulseinDegrees _player_2_3 (Math|Vector|MakeVector 0.0 0.0 (* _returnvalue_2 (Input|AxisValues|Getp2right) (Variables|Default|Getturningspeed))) "None" true))
        (:then_3
          ;[1 1 1] Shoot
          (if (Variables|Default|Getp2%20shoot)
            (bind _returnvalue_8 (Game|SpawnActorfromClass "/Game/Blueprints/bullet.bullet_C" (Math|Transform|MakeTransform (Transformation|GetSocketLocation _player_2_2 "Bullet") _rotation _scale) "Undefined" 0 0))
            (Physics|AddImpulse (Variables|/Game/Blueprints/bullet.bullet_C|GetSphere _returnvalue_8) (* (Math|Vector|GetForwardVector _player_2_2) (Variables|Default|GetshootForce)) "None" true)
            (Variables|Default|Setp2%20shoot false)))))))

(event Input|ActionEvents|InputActionp1shoot
  (params (Key :type Key%20Structure))
  (:Pressed
    (Variables|Default|Setp1%20shoot true))
  (:Released
    (Variables|Default|Setp1%20shoot false)))

(event Input|ActionEvents|InputActionp2shoot
  (params (Key :type Key%20Structure))
  (:Pressed
    (Variables|Default|Setp2%20shoot true))
  (:Released
    (Variables|Default|Setp2%20shoot false)))

(fn ConstructionScript)

(fn SetStartTransforms
  (params (start1 :type Transform) (start2 :type Transform))
  (bind _output_get (Variables|Default|Setplayer1%20start start1))
  (bind _output_get_2 (Variables|Default|Setplayer2%20start start2))
  (Transformation|SetWorldTransform (Variables|Default|GetPlayer%201) _output_get false true)
  (Transformation|SetWorldTransform (Variables|Default|GetPlayer%202) _output_get_2 false true))