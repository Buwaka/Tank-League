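; Bumper Blueprint that applies impulses to components of the GameTraceChannel1 object type that overlap its Box.
; The impulse fires on begin overlap and again every Tick for each matching component still overlapping.
; It multiplies the Box's forward vector component-wise by the offset from the component to the Box, scales it by BumperStrength, and applies it as a mass-independent velocity change.
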(event OnComponentBeginOverlap(Box)
  (params (OverlappedComponent :type Primitive%20Component%20Object%20Reference) (OtherActor :type Actor%20Object%20Reference) (OtherComp :type Primitive%20Component%20Object%20Reference) (OtherBodyIndex :type Integer) (bFromSweep :type Boolean) (SweepResult :type Hit%20Result%20Structure%20%28by%20ref%29))
  (bind _box (Variables|Default|GetBox))
  (if (Utilities|Enum|Equal(Enum) (Collision|GetCollisionObjectType OtherComp) "ECC_GameTraceChannel1")
    (Physics|AddImpulse OtherComp (* (* (Math|Vector|GetForwardVector _box) (- (Transformation|GetWorldLocation _box) (Transformation|GetWorldLocation OtherComp))) (Variables|Default|Getbumper%20strength)) "None" true)))

(event EventTick
  (params (DeltaSeconds :type Float%20%28single-precision%29))
  (bind _box (Variables|Default|GetBox))
  (bind _box_2 (Variables|Default|GetBox))
  (bind _outoverlappingcomponents (Class|PrimitiveComponent|GetOverlappingComponents _box_2))
  (if (> (Utilities|Array|Length _outoverlappingcomponents) 0)
    (for _array_element _outoverlappingcomponents
      (if (Utilities|Enum|Equal(Enum) (Collision|GetCollisionObjectType _array_element) "ECC_GameTraceChannel1")
        (Physics|AddImpulse _array_element (* (* (Math|Vector|GetForwardVector _box) (- (Transformation|GetWorldLocation _box) (Transformation|GetWorldLocation _array_element))) (Variables|Default|Getbumper%20strength)) "None" true)))))

(fn ConstructionScript)