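; Game mode for a tank game that sets up the tank at match start and keeps per-team scores.
; On BeginPlay it spawns a single TankUnit at the "p1" player start, owned by that start.
; It then passes the "p1" and "p2" start transforms to the unit through SetStartTransforms.
; The Score function increments the Scores entry for the given team index.
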(event EventBeginPlay
  (bind _returnvalue (Game|GetPlayerController 0))
  (bind _returnvalue_2 (Class|GameModeBase|FindPlayerStart _returnvalue "p1"))
  (bind _returnvalue_3 (Transformation|GetActorTransform _returnvalue_2))
  (Utilities|FlowControl|Sequence
    (:then_0
      (bind _returnvalue_4 (Game|SpawnActorfromClass "/Game/Blueprints/TankUnit.TankUnit_C" _returnvalue_3 "Undefined" _returnvalue_2 0))
      (Default|SetStartTransforms _returnvalue_4 _returnvalue_3 (Transformation|GetActorTransform (Class|GameModeBase|FindPlayerStart (Game|GetPlayerController 1) "p2"))))))

(fn ConstructionScript)

(fn Score
  (params (Team%20index :type Integer))
  (Math|Integer|IncrementInt (Utilities|Array|Get(acopy) (Variables|Default|Getscores) Team%20index)))