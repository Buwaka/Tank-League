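; HUDManager is a Blueprint that creates and updates the TankLeagueHUD widget for the tank league game.
; On BeginPlay it adds the HUD to the first player's viewport, stores a reference, and passes the game mode's countdown duration to its countdown.
; SetScore writes both players' scores directly into the widget's score variables.
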(event EventBeginPlay
  (bind _returnvalue (UserInterface|CreateWidget "/Game/Blueprints/TankLeagueHUD.TankLeagueHUD_C" (Game|GetPlayerController 0)))
  (UserInterface|Viewport|AddtoViewport _returnvalue 0)
  (Variables|Default|SetHUD%20widget _returnvalue)
  (bind _astankgamemode (Utilities|Casting|CastTotankgamemode (Game|GetGameMode)))
  (Default|SetCountdown (Variables|Default|GetHUD%20widget) (Math|Conversions|ToFloat(Integer) (Variables|/Game/Blueprints/tankgamemode.tankgamemode_C|GetCountdown%20duration _astankgamemode))))

(fn ConstructionScript)

(fn SetScore
  (params (p1 :type Integer) (p2 :type Integer))
  (bind _hud_widget (Variables|Default|GetHUD%20widget))
  (Variables|/Game/Blueprints/TankLeagueHUD.TankLeagueHUD_C|Setp1%20score _hud_widget p1)
  (Variables|/Game/Blueprints/TankLeagueHUD.TankLeagueHUD_C|Setp2%20score _hud_widget p2))