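; Game mode for a two-player tank game that spawns the tank actor, tracks round scores and ends the match.
; SpawnPlayers creates a single TankUnit at the "p1" start and hands it both start transforms.
; Score credits a team, shows the WinScreen widget once the round limit is reached and updates the HUDManager.
; Spawning and scoring both trigger a countdown delay that disables the tank's input for player controller 0.
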(event Custom|temporarily%20disable%20%20player%20input
  (bind _returnvalue (Game|GetPlayerController 0))
  (bind _tank_pawn (Variables|Default|Gettank%20pawn))
  (Input|DisableInput _tank_pawn _returnvalue)
  (Utilities|FlowControl|Delay (Math|Conversions|ToFloat(Integer) (Variables|Default|GetCountdown%20duration)))
  (Input|EnableInput _tank_pawn _returnvalue))

(fn ConstructionScript)

(fn Score
  (params (Team%20index :type Integer))
  (switch int Team%20index
    (:0
      (bind _result (Math|Integer|IncrementInt (Variables|Default|Getp1%20score))
        (:%20%20
          _)))
    (:1
      (bind _result_2 (Math|Integer|IncrementInt (Variables|Default|Getp2%20score))
        (:%20%20
          _))))
  (bind _result_3 (Math|Integer|IncrementInt (Variables|Default|Getrounds))
    (:%20%20
      (if (>= _result_3 (Variables|Default|GetRoundCount))
        (bind _returnvalue (UserInterface|CreateWidget "/Game/Blueprints/WinScreen.WinScreen_C" (Game|GetPlayerController 0)))
        (Default|Winner _returnvalue (Variables|Default|Getp1%20score) (Variables|Default|Getp2%20score))
        (UserInterface|Viewport|AddtoViewport _returnvalue 0))
      (bind _ashudmanager (Utilities|Casting|CastToHUDManager (HUD|GetHUD (Game|GetPlayerController 0))))
      (Default|SetScore _ashudmanager _result _result_2)
      (CallFunction|TemporarilyDisablePlayerInput))))

(fn SpawnPlayers
  (bind _returnvalue (Game|GetPlayerController 0))
  (bind _returnvalue_2 (Class|GameModeBase|FindPlayerStart _returnvalue "p1"))
  (bind _returnvalue_3 (Transformation|GetActorTransform _returnvalue_2))
  (Utilities|FlowControl|Sequence
    (:then_0
      (bind _returnvalue_4 (Game|SpawnActorfromClass "/Game/Blueprints/TankUnit.TankUnit_C" _returnvalue_3 "Undefined" _returnvalue_2 0))
      (bind _output_get (Variables|Default|Settank%20pawn _returnvalue_4))
      (Default|SetStartTransforms _output_get _returnvalue_3 (Transformation|GetActorTransform (Class|GameModeBase|FindPlayerStart (Game|GetPlayerController 0) "p2")))
      (CallFunction|TemporarilyDisablePlayerInput))))