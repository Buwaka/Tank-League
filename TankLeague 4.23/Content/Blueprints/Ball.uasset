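; Ball actor whose sphere mesh can play a scale-up "explosion" and then be reset.
; Explode sets a duration and starts a timer in Tick that lerps the sphere from its starting scale toward a size multiplier.
; Once the duration passes, the sphere is hidden; Reset clears the timer, restores the original scale and shows it again.
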(event EventBeginPlay
  (Variables|Default|Setstart%20scale (Transformation|GetWorldScale (Variables|Default|GetSphere))))

(event Collision|EventActorBeginOverlap
  (params (OtherActor :type Actor%20Object%20Reference)))

(event EventTick
  (params (DeltaSeconds :type Float%20%28single-precision%29))
  (if (Variables|Default|GetIsexploding)
    (bind _output_get (Variables|Default|Settimer (+ DeltaSeconds (Variables|Default|Gettimer))))
    (Transformation|SetWorldScale3D (Variables|Default|GetSphere) (* (Variables|Default|Getstart%20scale) (Math|Float|Lerp 1.0 (Variables|Default|Getexplosion%20size%20scale) (/ _output_get (Variables|Default|Getexplosion%20time)))))
    (if (> (/ _output_get (Variables|Default|Getexplosion%20time)) 1.0)
      (Development|SetHiddeninGame (Variables|Default|GetSphere) true false))))

(fn ConstructionScript)

(fn Explode
  (params (duration :type Float%20%28single-precision%29))
  (Variables|Default|SetIsexploding true)
  (Variables|Default|Setexplosion%20time duration))

(fn Reset
  (Variables|Default|SetIsexploding false)
  (Variables|Default|Settimer 0.0)
  (Transformation|SetWorldScale3D (Variables|Default|GetSphere) (Variables|Default|Getstart%20scale))
  (Development|SetHiddeninGame (Variables|Default|GetSphere) false false))