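; Bumper Blueprint that pushes physics components of the GameTraceChannel1 object type out along its Box's forward vector.
; An impulse fires when a component begins overlapping the Box and again every Tick while it stays inside.
; The forward vector is multiplied per axis by the absolute offset between component and Box, then by BumperStrength, so the push grows with distance from the Box origin.
; Impulses apply as velocity changes, ignoring mass.
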(event OnComponentBeginOverlap(Box)
  (params (OverlappedComponent :type Primitive%20Component%20Object%20Reference) (OtherActor :type Actor%20Object%20Reference) (OtherComp :type Primitive%20Component%20Object%20Reference) (OtherBodyIndex :type Integer) (bFromSweep :type Boolean) (SweepResult :type Hit%20Result%20Structure%20%28by%20ref%29))
  (bind _box (Variables|Default|GetBox))
  (bind _distance (CallFunction|AbsoluteDistanceBetweenComponents _box OtherComp))
  (if (Utilities|Enum|Equal(Enum) (Collision|GetCollisionObjectType OtherComp) "ECC_GameTraceChannel1")
    (Physics|AddImpulse OtherComp (* (* (Math|Vector|GetForwardVector _box) _distance) (Variables|Default|Getbumper%20strength)) "None" true)))

(event EventTick
  (params (DeltaSeconds :type Float%20%28single-precision%29))
  (bind _box (Variables|Default|GetBox))
  (bind _box_2 (Variables|Default|GetBox))
  (bind _outoverlappingcomponents (Class|PrimitiveComponent|GetOverlappingComponents _box))
  (if (> (Utilities|Array|Length _outoverlappingcomponents) 0)
    (for _array_element _outoverlappingcomponents
      (bind _distance (CallFunction|AbsoluteDistanceBetweenComponents _box_2 _array_element))
      (if (Utilities|Enum|Equal(Enum) (Collision|GetCollisionObjectType _array_element) "ECC_GameTraceChannel1")
        (Physics|AddImpulse _array_element (* (* (Math|Vector|GetForwardVector _box_2) _distance) (Variables|Default|Getbumper%20strength)) "None" true)))))

(fn ConstructionScript)

(fn AbsoluteDistanceBetweenComponents
  (params (obj1 :type Primitive%20Component%20Object%20Reference) (obj2 :type Primitive%20Component%20Object%20Reference))
  (bind _returnvalue (Transformation|GetWorldLocation obj2))
  (bind _returnvalue_2 (Transformation|GetWorldLocation obj1))
  (bind _returnvalue_3 (- _returnvalue_2 _returnvalue))
  (bind (_x _y _z) (Math|Vector|BreakVector _returnvalue_3))
  (return (Math|Vector|MakeVector (Math|Float|Absolute(Float) _x) (Math|Float|Absolute(Float) _y) (Math|Float|Absolute(Float) _z))))