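; Goal actor that registers a score when a Ball enters its Box trigger.
; On overlap it explodes the ball with a value scaled from TimeBeforeNextRound and passes its Teamindex to the tankgamemode's Score.
; It then plays a world camera shake with a very large radius and, after the TimeBeforeNextRound delay, has the game mode reset the level.
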(event OnComponentBeginOverlap(Box)
  (params (OverlappedComponent :type Primitive%20Component%20Object%20Reference) (OtherActor :type Actor%20Object%20Reference) (OtherComp :type Primitive%20Component%20Object%20Reference) (OtherBodyIndex :type Integer) (bFromSweep :type Boolean) (SweepResult :type Hit%20Result%20Structure%20%28by%20ref%29))
  (bind _returnvalue (Game|GetGameMode))
  (bind _time_before_next_round (Variables|Default|Gettime%20before%20next%20round))
  (bind _asball (Utilities|Casting|CastToBall OtherActor))
  (Default|Explode _asball (/ _time_before_next_round 1e+01))
  (bind _astankgamemode (Utilities|Casting|CastTotankgamemode _returnvalue))
  (Default|Score _astankgamemode (Variables|Default|Getteamindex))
  (Camera|PlayWorldCameraShake "/Game/Blueprints/ScoreShake.ScoreShake_C" "0, 0, 0" 0.0 1e+06 0.0)
  (Utilities|FlowControl|Delay _time_before_next_round)
  (Class|GameModeBase|ResetLevel _returnvalue))

(fn ConstructionScript)